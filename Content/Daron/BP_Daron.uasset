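; Daron is an enemy that hurts the player on contact and triggers the player's win when projectile hits deplete its health.
; It registers with the game instance, then each Tick drives its pitch and vertical bobbing from curves on a speed-scaled timer.
; A slowdown for stealth quarters that speed until its delay ends or it is interrupted.
; When stealth ends, it spawns an alert actor at an offset.
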(event `self.ReceiveBeginPlay`
  ;[1 1 1] BeginPlay, get initial location
  (set `self.BaseLocation` (`self.K2_GetActorLocation`))
  ;[1 1 1] Register to game instance
  (bind _asbp_game_instance (cast `/Game/BP_GameInstance` (`GameplayStatics.GetGameInstance`)))
  (set `/Game/BP_GameInstance.DaronObject` self _asbp_game_instance))

(event `self.ReceiveTick`
  (params (DeltaSeconds :type "Float (single-precision)"))
  (bind (_baselocation_x _baselocation_y _baselocation_z) (`KismetMathLibrary.BreakVector` (`self.BaseLocation`)))
  ;[1 1 1] Rotation
  (`self.K2_SetActorRotation` (`KismetMathLibrary.MakeRotator` 0.0 (`CurveFloat.GetFloatValue` (`self.RotationCurve`) (`self.RotationTimer`))))
  ;[1 1 1] Height variation
  (`self.K2_SetActorLocation` (`KismetMathLibrary.MakeVector` _baselocation_x _baselocation_y (+ _baselocation_z (`CurveFloat.GetFloatValue` (`self.HeightLocationCurve`) (`self.RotationTimer`)))))
  ;[1 1 1] Curve timer
  (set `self.RotationTimer` (+ (`self.RotationTimer`) (* DeltaSeconds (`self.RotationSpeed`)))))

(event `self.RenderComponent.OnComponentHit`
  (params (HitComponent :type "PrimitiveComponent Object Reference") (OtherActor :type "Actor Object Reference") (OtherComp :type "PrimitiveComponent Object Reference") (NormalImpulse :type "Vector Structure") (Hit :type "HitResult Structure (by ref)"))
  ;[1 1 1] Touching the played
  (bind _asbp_dice_player_controller (cast `/Game/Player/BP_DicePlayerController` OtherActor))
  (`/Game/Player/BP_DicePlayerController.OnHitByEnemy` _asbp_dice_player_controller))

(event `OnHitByProjectile`
  ;[1 1 1] Hit by proj
  (bind _result (`/Engine/EditorBlueprintResources/StandardMacros.DecrementInt` (`self.HealthPoints`))
    (:`  `
      (if (<= _result 0)
        (bind _asbp_dice_player_controller (cast `/Game/Player/BP_DicePlayerController` (`GameplayStatics.GetPlayerCharacter` 0)))
        (`/Game/Player/BP_DicePlayerController.OnWin` _asbp_dice_player_controller)))))

(event `OnInterruptSlowDown`
  ;[1 1 1] Slowdown for stealth
  (if (`self.IsInSlowdown`) :!label _label
    (set `self.RotationSpeed` (* (`self.RotationSpeed`) 4.0))
    (set `self.IsInSlowdown` false)))

(event `OnSlowDown`
  (params (Duration :type "Float (double-precision)"))
  ;[1 1 1] Slowdown for stealth
  (set `self.RotationSpeed` (* (`self.RotationSpeed`) 0.25))
  (set `self.IsInSlowdown` true)
  (`KismetSystemLibrary.Delay` Duration)
  (goto _label))

(event `OnStealthEnded`
  (bind (_returnvalue_x _returnvalue_y _returnvalue_z) (`KismetMathLibrary.BreakVector` (`self.K2_GetActorLocation`)))
  (`|SpawnActorFromClass` "/Game/Daron/BP_Alert.BP_Alert_C" (`KismetMathLibrary.MakeTransform` (`KismetMathLibrary.MakeVector` (+ _returnvalue_x 250.0) (+ _returnvalue_y 1.0) (+ _returnvalue_z 150.0)) (struct) (2.0 1.0 2.0)) "Undefined" "OverrideRootScale" null null))

(fn `UserConstructionScript`)