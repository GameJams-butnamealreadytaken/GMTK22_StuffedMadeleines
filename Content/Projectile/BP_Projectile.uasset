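; BP_Projectile is a flipbook-sprite projectile that moves along its Direction vector and can hit BP_Daron.
; Init mirrors the non-looping flipbook to match the X direction, and Tick moves the actor without sweeping, using Direction as velocity.
; On overlap it notifies BP_Daron if hit, then destroys itself and spawns BP_PiouHit, ignoring other projectiles and BP_DicePlayerController.
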(event `self.ReceiveBeginPlay`
  (`self.Init`))

(event `Init`
  (bind _direction_x (`KismetMathLibrary.BreakVector` (`self.Direction`)))
  (`SceneComponent.SetRelativeScale3D` (`self.PaperFlipbook`) (`KismetMathLibrary.MakeVector` (`KismetMathLibrary.SelectFloat` -1.0 1.0 (< _direction_x 0.0)) 1.0 1.0)))

(event `self.ReceiveTick`
  (params (DeltaSeconds :type "Float (single-precision)"))
  (`self.K2_SetActorLocation` (+ (* DeltaSeconds (`self.Direction`)) (`self.K2_GetActorLocation`))))

(event `self.ReceiveActorBeginOverlap`
  (params (OtherActor :type "Actor Object Reference"))
  (bind _returnvalue_location (`KismetMathLibrary.BreakTransform` (`self.GetTransform`)))
  (bind _asbp_daron (cast `/Game/Daron/BP_Daron` OtherActor)
    (:`then`
      (`/Game/Daron/BP_Daron.OnHitByProjectile` _asbp_daron))
    (:`CastFailed`
      (cast `/Game/Player/BP_DicePlayerController` OtherActor
        (:`CastFailed`
          (cast `/Game/Projectile/BP_Projectile` OtherActor
            (:`CastFailed`
              _))))))
  (`self.K2_DestroyActor`)
  (`|SpawnActorFromClass` "/Game/Projectile/BP_PiouHit.BP_PiouHit_C" (`KismetMathLibrary.MakeTransform` _returnvalue_location) "AlwaysSpawn" "OverrideRootScale" null null))

(fn `UserConstructionScript`
  (`PaperFlipbookComponent.SetLooping` (`self.PaperFlipbook`) false))