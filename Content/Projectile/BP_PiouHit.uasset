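; BP_PiouHit is a projectile hit effect, shown as a one-shot Paper2D flipbook animation.
; Each tick it teleports backward along X by the RunnerManager's BlockMoveSpeed from BP_GameInstance, scaled by delta time, so it scrolls at the runner's block speed.
; The construction script disables looping, and the actor destroys itself when the flipbook finishes playing.
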(event `self.ReceiveTick`
  (params (DeltaSeconds :type "Float (single-precision)"))
  (bind _returnvalue (`self.GetTransform`))
  (bind _asbp_game_instance (cast `/Game/BP_GameInstance` (`GameplayStatics.GetGameInstance`)))
  (`self.K2_TeleportTo` (`KismetMathLibrary.MakeVector` (+ (* (`/Game/Runner/BP_RunnerManager.BlockMoveSpeed` (`/Game/BP_GameInstance.RunnerManager` _asbp_game_instance)) DeltaSeconds -1.0) (.x (.location _returnvalue))) (.y (.location _returnvalue)) (.z (.location _returnvalue)))))

(event `self.PaperFlipbook.OnFinishedPlaying`
  (`self.K2_DestroyActor`))

(fn `UserConstructionScript`
  (`PaperFlipbookComponent.SetLooping` (`self.PaperFlipbook`) false))