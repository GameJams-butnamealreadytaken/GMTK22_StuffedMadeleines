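; Runner manager that procedurally generates and scrolls the side-scroller level of ground blocks, dice upgrades and traps, registering itself in the GameInstance.
; Tick moves all blocks and adds columns on a speed-based timer, following either random-walk heights or trap layouts.
; Traps are picked by randomized, recovering weights among those the player's available dice abilities allow.
; An overlap detector destroys passed blocks, and slow-down events temporarily scale scroll speed and spawn timing.
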(event `self.ReceiveBeginPlay`
  (`|ExecutionSequence`
    (:`then_0`
      ;[1 1 1] Set itself in gameinstance
      (bind _asbp_game_instance (cast `/Game/BP_GameInstance` (`GameplayStatics.GetGameInstance`)))
      (set `/Game/BP_GameInstance.RunnerManager` self _asbp_game_instance)
      (set `self.GroundHeight` (`self.MinHeightFloor`)))
    (:`then_1`
      ;[1 1 1] Generate first ground block
      (`self.CreateGroundBlocks`))
    (:`then_2`
      ;[1 1 1] Dice upgrade spawn rate
      (`KismetSystemLibrary.Delay` (`KismetMathLibrary.RandomFloatInRange` (`self.DiceUgradeSpawnRateMin`) (`self.DiceUgradeSpawnRateMax`)) :!label _label)
      (set `self.SpawnDiceUpgrade` true)
      (goto _label))
    (:`then_3`
      ;[1 1 1] Init trap ponderations
      (for _array_element (`self.TrapList`)
        (`KismetArrayLibrary.Array_Add` (`self.TrapPonderation`) (`/Game/Runner/Trap/BP_TrapDataAsset.ChancesToAppear` _array_element))))
    (:`then_4`
      (`self.GenerateGroundBlocksAtStart`))))

(event `self.ReceiveTick`
  (params (DeltaSeconds :type "Float (single-precision)"))
  (bind _trapponderation (`self.TrapPonderation`))
  (bind _trapponderation_2 (`self.TrapPonderation`))
  (bind _output (`|GetArrayItem` (`self.TrapList`) (`self.CurrentGeneratedTrap`)))
  (bind (_trapblockheights _neededgroundfromcurrentheight _neededgroundfromminheight _useminheightreferencial) (break `/Game/Runner/Trap/STR_TrapColumn` (`|GetArrayItem` (`/Game/Runner/Trap/BP_TrapDataAsset.TrapColumns` (`|GetArrayItem` (`self.TrapList`) (`self.CurrentGeneratedTrap`))) (`self.CurrentTrapColumnCounter`))))
  (bind (_trapblockheights_2 _neededgroundfromcurrentheight_2 _neededgroundfromminheight_2 _useminheightreferencial_2) (break `/Game/Runner/Trap/STR_TrapColumn` (`|GetArrayItem` (`/Game/Runner/Trap/BP_TrapDataAsset.TrapColumns` (`|GetArrayItem` (`self.TrapList`) (`self.CurrentGeneratedTrap`))) (`self.CurrentTrapColumnCounter`))))
  ;[1 1 1] Move blocks
  (for _array_element (`self.RunnerBlockList`)
    (bind (_returnvalue_x _returnvalue_y _returnvalue_z) (`KismetMathLibrary.BreakVector` (`self.K2_GetActorLocation` _array_element)))
    (`self.K2_SetActorLocation` _array_element (`KismetMathLibrary.MakeVector` (- _returnvalue_x (* DeltaSeconds (`self.BlockMoveSpeed`))) _returnvalue_y _returnvalue_z) false false))
  ;[1 1 1] Check if can generate next column (+ trap timer update)
  (set `self.LastTrapTimer` (+ DeltaSeconds (`self.LastTrapTimer`)))
  (bind _output_get (set `self.LastBlockTimer` (+ DeltaSeconds (`self.LastBlockTimer`))))
  (if (>= _output_get (/ 62.0 (`self.BlockMoveSpeed`)))
    ;[1 1 1] Check if not generating a trap
    (if (not (== (`self.CurrentGeneratedTrap`) -1))
      ;[1 1 1] Create trap blocks
      (`self.CreateTrapBlocks` (`.TrapBlockHeights_3_0745A47247B48E2FA17CEF8483C9B6E8` (break `/Game/Runner/Trap/STR_TrapColumn` (`|GetArrayItem` (`/Game/Runner/Trap/BP_TrapDataAsset.TrapColumns` _output) (`self.CurrentTrapColumnCounter`)))) (`/Game/Runner/Trap/BP_TrapDataAsset.DicePower` _output))
      (set `self.CurrentTrapColumnCounter` (+ (`self.CurrentTrapColumnCounter`) 1)))
    ;[1 1 1] Ground block creation
    (bind _highestcreatedbock (`self.CreateGroundBlocks`))
    ;[1 1 1] Check if not generating a trap
    (if (== (`self.CurrentGeneratedTrap`) -1)
      ;[1 1 1] Create Dice upgrade if needed
      (if (`self.SpawnDiceUpgrade`)
        (`self.createDiceUpgradeCollectible` _highestcreatedbock)
        ;[1 1 1] Chose next ground block height
        (set `self.GroundHeight` (`KismetMathLibrary.Clamp` (+ (`KismetMathLibrary.RandomIntegerInRange` -1 1) (`self.GroundHeight`)) (`self.MinHeightFloor`) (`self.MaxHeightFloor`)) :!label _label_2)
        (else
          ;[1 1 1] Check if can generate a trap instead
          (if (and (== (`self.CurrentGeneratedTrap`) -1) (>= (`self.LastTrapTimer`) (`self.TrapNextSpawnTime`)))
            (bind _trapid (`self.Get Trap IDTo Generate`))
            (if (!= _trapid -1)
              (set `self.CurrentGeneratedTrap` _trapid)
              (set `self.CurrentTrapColumnCounter` 0)
              (set `self.GroundHeight` (`KismetMathLibrary.SelectInt` (+ _neededgroundfromminheight_2 (`self.MinHeightFloor`)) (+ _neededgroundfromcurrentheight_2 (`self.GroundHeight`)) _useminheightreferencial_2))
              (`KismetArrayLibrary.Array_Set` _trapponderation (`self.CurrentGeneratedTrap`) (* (`|GetArrayItem` _trapponderation (`self.CurrentGeneratedTrap`)) 0.25))
              (else
                (goto _label_2)))
            (else
              (goto _label_2)))))
      (else
        ;[1 1 1] End of trap check
        (if (`KismetArrayLibrary.Array_IsValidIndex` (`/Game/Runner/Trap/BP_TrapDataAsset.TrapColumns` (`|GetArrayItem` (`self.TrapList`) (`self.CurrentGeneratedTrap`))) (`self.CurrentTrapColumnCounter`))
          (set `self.GroundHeight` (`KismetMathLibrary.SelectInt` (+ _neededgroundfromminheight (`self.MinHeightFloor`)) (+ _neededgroundfromcurrentheight (`self.GroundHeight`)) _useminheightreferencial))
          (else
            (set `self.CurrentGeneratedTrap` -1)
            (set `self.LastTrapTimer` 0.0)
            (set `self.TrapNextSpawnTime` (`KismetMathLibrary.RandomFloatInRange` (`self.TrapSpawnRateMin`) (`self.TrapSpawnRateMax`)))
            (for (_array_element_2 _array_index) _trapponderation_2
              (`KismetArrayLibrary.Array_Set` _trapponderation_2 _array_index (`KismetMathLibrary.FMin` (+ _array_element_2 0.1) (`/Game/Runner/Trap/BP_TrapDataAsset.ChancesToAppear` (`|GetArrayItem` (`self.TrapList`) _array_index)))))))))))

(event `self.DestroyDetector.OnComponentBeginOverlap`
  (params (OverlappedComponent :type "PrimitiveComponent Object Reference") (OtherActor :type "Actor Object Reference") (OtherComp :type "PrimitiveComponent Object Reference") (OtherBodyIndex :type Integer) (bFromSweep :type Boolean) (SweepResult :type "HitResult Structure (by ref)"))
  ;[1 1 1] Destroy blocks when reaching the limit
  (bind _aspaper_sprite_actor (cast `PaperSpriteActor` OtherActor))
  (`KismetArrayLibrary.Array_RemoveItem` (`self.RunnerBlockList`) _aspaper_sprite_actor)
  (`self.K2_DestroyActor` _aspaper_sprite_actor))

(event `DestroyRunnerBlock`
  (params (BlockToDestroy :type "PaperSpriteActor Object Reference"))
  ;[1 1 1] Destroy given block
  (`KismetArrayLibrary.Array_RemoveItem` (`self.RunnerBlockList`) BlockToDestroy)
  (`self.K2_DestroyActor` BlockToDestroy))

(event `OnInterruptSlowDown`
  ;[1 1 1] Slow down!
  (if (`self.IsInSlowdown`) :!label _label_3
    (set `self.BlockMoveSpeed` (* (`self.BlockMoveSpeed`) 4.0))
    (set `self.LastBlockTimer` (* (`self.LastBlockTimer`) 0.25))
    (set `self.IsInSlowdown` false)))

(event `OnSlowDown`
  (params (Duration :type "Float (double-precision)"))
  ;[1 1 1] Slow down!
  (set `self.BlockMoveSpeed` (* (`self.BlockMoveSpeed`) 0.25))
  (set `self.LastBlockTimer` (* (`self.LastBlockTimer`) 4.0))
  (set `self.IsInSlowdown` true)
  (`KismetSystemLibrary.Delay` Duration)
  (goto _label_3))

(fn `createDiceUpgradeCollectible`
  (params (LastCreatedBlock :type "PaperSpriteActor Object Reference"))
  (locals (DiceID :type Integer))
  (bind (_returnvalue_x _returnvalue_y _returnvalue_z) (`KismetMathLibrary.BreakVector` (`self.K2_GetActorLocation` LastCreatedBlock)))
  ;[1 1 1] Get a random dice ID that the player doesn't already have
  (bind _asbp_dice_player_controller (cast `/Game/Player/BP_DicePlayerController` (`GameplayStatics.GetPlayerCharacter` 0)))
  (bind _missingdiceids (`/Game/Player/BP_DicePlayerController.GetMissingDicesList` _asbp_dice_player_controller))
  (bind _returnvalue (`KismetArrayLibrary.Array_Length` _missingdiceids))
  (if (> _returnvalue 0)
    (bind _output_get (set `local.DiceID` (`|GetArrayItem` _missingdiceids (`KismetMathLibrary.RandomInteger` _returnvalue))))
    ;[1 1 1] Avoid generating dice 20 if not the last
    (bind _number (`/Game/Player/BP_DicePlayerController.IdToDiceNumber` _asbp_dice_player_controller _output_get))
    (if (or (!= _number 20) (== _returnvalue 1))
      (bind _returnvalue_2 (`|SpawnActorFromClass` (`self.DiceUpgrade`) (`KismetMathLibrary.MakeTransform` (`KismetMathLibrary.MakeVector` _returnvalue_x (+ _returnvalue_y 0.5) (+ _returnvalue_z 45.0))) "Undefined" "OverrideRootScale" null null))
      (bind _asbp_dice_upgrade_collectible (cast `/Game/Runner/Collectibles/BP_DiceUpgradeCollectible` _returnvalue_2))
      (`/Game/Runner/Collectibles/BP_DiceUpgradeCollectible.InitDiceUpgrade` _asbp_dice_upgrade_collectible (`local.DiceID`) self)
      (`KismetArrayLibrary.Array_Add` (`self.RunnerBlockList`) _returnvalue_2)
      (set `self.SpawnDiceUpgrade` false :!label _label))
    (else
      (goto _label))))

(fn `CreateGroundBlocks`
  (returns (HighestCreatedBock :type "PaperSpriteActor Object Reference"))
  (locals (LastAddedBlock :type "PaperSpriteActor Object Reference"))
  (bind (_returnvalue_x _returnvalue_y _returnvalue_z) (`KismetMathLibrary.BreakVector` (`self.K2_GetActorLocation`)))
  (for _index (range (`self.MinHeightFloor`) (+ (`self.GroundHeight`) 1))
    (bind _returnvalue (`|SpawnActorFromClass` (`self.GroundBlockSprite`) (`KismetMathLibrary.MakeTransform` (`KismetMathLibrary.MakeVector` (- _returnvalue_x 0.0) (- _returnvalue_y 0.5) (+ _returnvalue_z (`KismetMathLibrary.Conv_IntToDouble` (* _index (`self.BlockSize`)))))) "Undefined" "OverrideRootScale" null null))
    (`KismetArrayLibrary.Array_Add` (`self.RunnerBlockList`) _returnvalue)
    (set `local.LastAddedBlock` _returnvalue))
  (set `self.LastBlockTimer` 0.0)
  (return (`local.LastAddedBlock`)))

(fn `CreateTrapBlocks`
  (params (HeightList :type "Array of Integer") (DiceId :type Integer))
  (bind (_returnvalue_x _returnvalue_y _returnvalue_z) (`KismetMathLibrary.BreakVector` (`self.K2_GetActorLocation`)))
  (for _array_element HeightList
    (bind _returnvalue (`|SpawnActorFromClass` (`self.TrapBlockSprite`) (`KismetMathLibrary.MakeTransform` (`KismetMathLibrary.MakeVector` _returnvalue_x (- _returnvalue_y 0.5) (+ _returnvalue_z (`KismetMathLibrary.Conv_IntToDouble` (* (+ _array_element (`self.GroundHeight`)) 64))))) "Undefined" "OverrideRootScale" null null))
    (`KismetArrayLibrary.Array_Add` (`self.RunnerBlockList`) _returnvalue)
    (bind _asbp_trap_block (cast `/Game/Runner/Blocks/BP_TrapBlock` _returnvalue))
    (`/Game/Runner/Blocks/BP_TrapBlock.SetBlockDiceType` _asbp_trap_block DiceId))
  (return))

(fn `GenerateGroundBlocksAtStart`
  (locals (CurrentSpawnX :type "Float (double-precision)"))
  (bind _returnvalue_x (`KismetMathLibrary.BreakVector` (`self.K2_GetActorLocation`)))
  (bind (_returnvalue_x_2 _returnvalue_y _returnvalue_z) (`KismetMathLibrary.BreakVector` (`self.K2_GetActorLocation`)))
  (bind _returnvalue_x_3 (`KismetMathLibrary.BreakVector` (`SceneComponent.K2_GetComponentLocation` (`self.DestroyDetector`))))
  (for _index (range (+ (`KismetMathLibrary.FTrunc` (/ (`KismetMathLibrary.Abs` (- _returnvalue_x_3 _returnvalue_x)) (`self.BlockSize`))) 1))
    (bind _returnvalue (`|SpawnActorFromClass` (`self.GroundBlockSprite`) (`KismetMathLibrary.MakeTransform` (`KismetMathLibrary.MakeVector` (- _returnvalue_x_2 (* (`self.BlockSize`) _index)) (- _returnvalue_y 0.5) (+ _returnvalue_z (`KismetMathLibrary.Conv_IntToDouble` (* (`self.BlockSize`) (`self.MinHeightFloor`)))))) "Undefined" "OverrideRootScale" null null))
    (`KismetArrayLibrary.Array_Add` (`self.RunnerBlockList`) _returnvalue)))

(fn `Get Trap IDTo Generate`
  (returns (TrapID :type Integer))
  (locals (AvailableTrapIDs :type "Array of Integer") (TrapChanceValues :type "Array of Float (double-precision)"))
  (bind _asbp_dice_player_controller (cast `/Game/Player/BP_DicePlayerController` (`GameplayStatics.GetPlayerCharacter` 0))
    (:`then`
      (for (_array_element _array_index) (`self.TrapList`)
        (switch `int` (`/Game/Runner/Trap/BP_TrapDataAsset.DicePower` _array_element)
          (:`4`
            (`KismetArrayLibrary.Array_Add` (`local.AvailableTrapIDs`) _array_index :!label _label))
          (:`6`
            (bind _newparam (`/Game/Player/BP_DicePlayerController.CanDoubleJump` _asbp_dice_player_controller))
            (if _newparam
              (goto _label)))
          (:`8`
            (bind _newparam_2 (`/Game/Player/BP_DicePlayerController.CanSlowDown` _asbp_dice_player_controller))
            (if _newparam_2
              (bind _newparam_3 (`/Game/Player/BP_DicePlayerController.IsSlowDownCoolingDown` _asbp_dice_player_controller))
              (if (not _newparam_3)
                (goto _label))))
          (:`10`
            (bind _newparam_4 (`/Game/Player/BP_DicePlayerController.CanDash` _asbp_dice_player_controller))
            (if _newparam_4
              (bind _newparam_5 (`/Game/Player/BP_DicePlayerController.IsDashCoolingDown` _asbp_dice_player_controller))
              (if (not _newparam_5)
                (goto _label))))
          (:`12`
            (bind _newparam_6 (`/Game/Player/BP_DicePlayerController.CanStealth` _asbp_dice_player_controller))
            (if _newparam_6
              (bind _newparam_7 (`/Game/Player/BP_DicePlayerController.IsStealthCoolingDown` _asbp_dice_player_controller))
              (if (not _newparam_7)
                (goto _label))))))
      (for _array_element_2 (`local.AvailableTrapIDs`)
        (`KismetArrayLibrary.Array_Add` (`local.TrapChanceValues`) (* (`|GetArrayItem` (`self.TrapPonderation`) _array_element_2) (`KismetMathLibrary.RandomFloatInRange` 1.0 2.0))))
      (return (`|GetArrayItem` (`local.AvailableTrapIDs`) (`KismetMathLibrary.MaxOfFloatArray` (`local.TrapChanceValues`)))))
    (:`CastFailed`
      (return -1))))

(fn `UserConstructionScript`)