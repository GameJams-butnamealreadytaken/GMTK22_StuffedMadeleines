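; Runner collectible that grants the player a dice upgrade identified by a DiceID.
; InitDiceUpgrade stores the ID and runner manager, then sets the sprite for that die.
; OnPlayerHit passes the ID to the player's OnDiceUpgradeCollected and has the manager destroy the block.
; A render component overlap with BP_Daron also destroys the block through the manager, without granting the upgrade itself.
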(event `InitDiceUpgrade`
  (params (DiceID :type Integer) (RunnerManager :type "/Game/Runner/BP_RunnerManager Object Reference"))
  (bind _output_get (set `self.DiceID` DiceID))
  (set `self.RunnerManagerRef` RunnerManager)
  (`PaperSpriteComponent.SetSprite` (`self.RenderComponent`) (`|GetArrayItem` (`self.DiceSprites`) _output_get)))

(event `self.ReceiveBeginPlay`
  (`parent.ReceiveBeginPlay`))

(event `self.RenderComponent.OnComponentBeginOverlap`
  (params (OverlappedComponent :type "PrimitiveComponent Object Reference") (OtherActor :type "Actor Object Reference") (OtherComp :type "PrimitiveComponent Object Reference") (OtherBodyIndex :type Integer) (bFromSweep :type Boolean) (SweepResult :type "HitResult Structure (by ref)"))
  (cast `/Game/Daron/BP_Daron` OtherActor)
  (`/Game/Runner/BP_RunnerManager.DestroyRunnerBlock` (`self.RunnerManagerRef`) self))

(fn `OnPlayerHit`
  (params (Player :type "/Game/Player/BP_DicePlayerController Object Reference"))
  (`/Game/Player/BP_DicePlayerController.OnDiceUpgradeCollected` Player (`self.DiceID`))
  (`/Game/Runner/BP_RunnerManager.DestroyRunnerBlock` (`self.RunnerManagerRef`) self))

(fn `UserConstructionScript`
  (`parent.UserConstructionScript`))