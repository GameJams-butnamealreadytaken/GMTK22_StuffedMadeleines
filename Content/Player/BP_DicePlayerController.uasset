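; Player character for a side-scrolling flipbook game, swapping between collected dice that change body shape and ability (jump boost, slow-down, dash, stealth, projectile).
; UseCurrentSkill fires the active die's power, while Tick runs timers and feeds cooldowns to the HUD.
; Enemy hits remove the current die and respawn the player, or end the game on the last one.
; Pickups and hits rescale global time dilation by dice count.
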(event `InputAction|Pause` :paused true
  (params (Key :type "Key Structure"))
  (bind _endscreen (`self.EndScreen`))
  ;[1 1 1] Added pause
  (:`Pressed`
    (`GameplayStatics.SetGamePaused` (not (`GameplayStatics.IsGamePaused`)))
    (if (`GameplayStatics.IsGamePaused`)
      (`/Game/UI/Bp_EndScreen.OnShow` _endscreen)
      (`/Game/UI/Bp_EndScreen.OnPause` _endscreen)
      (else
        (`/Game/UI/Bp_EndScreen.OnUnPause` _endscreen)))))

(event `self.ReceiveTick`
  (params (DeltaSeconds :type "Float (single-precision)"))
  (bind _stealthcurrenttime (`self.StealthCurrentTime`))
  (bind _rightarm (`self.RightArm`))
  (bind _dashcurrenttime (`self.DashCurrentTime`))
  (bind _leftarm (`self.LeftArm`))
  (bind _charactermovement (`self.CharacterMovement`))
  (bind _value (`BlueprintMapLibrary.Map_Find` (`self.DiceParametersArray`) 10))
  ;[1 1 1] Legs
  (if (not (> (`self.DashCurrentTime`) 0.0))
    (`PaperFlipbookComponent.SetFlipbook` (`self.Sprite`) (select `bool` (`NavMovementComponent.IsFalling` (`self.CharacterMovement`)) :`false` "/Game/Dice_sprite/FB_Legs.FB_Legs" :`true` "/Game/Dice_sprite/FB_JumpLegs.FB_JumpLegs" :!type "PaperFlipbook Object Reference")))
  (`self.UpdateCooldowns` DeltaSeconds)
  ;[1 1 1] Dash
  (if (> _dashcurrenttime 0.0)
    (bind _output_get (set `self.DashCurrentTime` (- _dashcurrenttime DeltaSeconds)))
    (if (not (> _output_get 0.0))
      (`MovementComponent.StopMovementImmediately` _charactermovement)
      (set `CharacterMovementComponent.GravityScale` 1.0 _charactermovement)
      (`PaperFlipbookComponent.SetFlipbook` (`self.Sprite`) "/Game/Dice_sprite/FB_Legs.FB_Legs")
      (`SceneComponent.K2_SetRelativeLocation` (`self.Sprite`) (`.LegPostion_21_4465FA6C4BA7FE0268173FB8DA4CB8B8` (break `/Game/Player/DiceParameters` _value)) false false)
      (`PaperFlipbookComponent.SetFlipbook` _leftarm "/Game/Dice_sprite/FB_LeftArm.FB_LeftArm")
      (`SceneComponent.K2_SetRelativeLocation` _leftarm (break `/Game/Player/DiceParameters` _value) false false)
      (`PaperFlipbookComponent.SetFlipbook` _rightarm "/Game/Dice_sprite/FB_RightArm.FB_RightArm")
      (`SceneComponent.K2_SetRelativeLocation` _rightarm (`.RightArmPosition_9_4A7DAD8C4587A3831790768D12833F1F` (break `/Game/Player/DiceParameters` _value)) false false)))
  ;[1 1 1] Stealth
  (if (> _stealthcurrenttime 0.0)
    (bind _output_get_2 (set `self.StealthCurrentTime` (- _stealthcurrenttime DeltaSeconds)))
    (if (not (> _output_get_2 0.0))
      (`SceneComponent.SetVisibility` (`self.Box`) false true)
      (`PrimitiveComponent.SetCollisionResponseToChannel` (`self.CapsuleComponent`) "ECC_GameTraceChannel2" "ECR_Block")
      (bind _asbp_game_instance (cast `/Game/BP_GameInstance` (`GameplayStatics.GetGameInstance`)))
      (`/Game/Daron/BP_Daron.OnStealthEnded` (`/Game/BP_GameInstance.DaronObject` _asbp_game_instance)))))

(event `OnDiceUpgradeCollected`
  (params (DiceID :type Integer))
  ;[1 1 1] Collected a dice upgrade
  (bind _number (`self.IdToDiceNumber` DiceID))
  (`self.GainDice` _number)
  (`GameplayStatics.SetGlobalTimeDilation` (+ (* 0.15 (`KismetArrayLibrary.Array_Length` (`self.AvailableDices`))) 0.9)))

(event `OnHitByEnemy`
  ;[1 1 1] Touched by an enemy
  (if (not (`self.IsInvulnarable`))
    (set `self.IsInvulnarable` true)
    (`self.Lose Current Dice`)
    (`self.K2_SetActorLocation` (`self.RespawnLoc`) false true)
    (`KismetSystemLibrary.Delay` 0.5)
    (set `self.IsInvulnarable` false)
    (`GameplayStatics.SetGlobalTimeDilation` (+ (* 0.15 (`KismetArrayLibrary.Array_Length` (`self.AvailableDices`))) 0.9))))

(event `self.ReceiveBeginPlay`
  ;[1 1 1] Begin play
  (bind _returnvalue (`|CreateWidget` "/Game/UI/BP_HUD.BP_HUD_C" (`GameplayStatics.GetPlayerController` 0)))
  (bind _output_get (set `self.HUD` _returnvalue))
  (`UserWidget.AddToViewport` _output_get 0)
  (for _array_element (`self.AvailableDices`)
    (`/Game/UI/BP_HUD.GainPower` (`self.HUD`) _array_element)
    (`self.SetDice` 4 :!label _label)
    (set `self.OriginalJumpZVelocity` (`CharacterMovementComponent.JumpZVelocity` (`self.CharacterMovement`)))
    (bind _returnvalue_2 (`|CreateWidget` "/Game/UI/Bp_EndScreen.Bp_EndScreen_C" (`GameplayStatics.GetPlayerController` 0)))
    (set `self.EndScreen` _returnvalue_2)
    (`GameplayStatics.SetGlobalTimeDilation` 1.0))
  (goto _label))

(event `InputAction|Jump`
  (params (Key :type "Key Structure"))
  ;[1 1 1] Inputs
  (:`Pressed`
    (`self.Jump`))
  (:`Released`
    (`self.StopJumping`)))

(event `InputAxis|Move`
  (params (AxisValue :type "Float (single-precision)"))
  (bind _returnvalue (`self.GetController`))
  ;[1 1 1] Inputs
  (if (<= (`self.DashCurrentTime`) 0.0)
    (`self.AddMovementInput` (1.0 0.0 0.0) AxisValue)
    (`/Engine/EditorBlueprintResources/StandardMacros.CompareFloat` AxisValue
      (:`>`
        (`Controller.SetControlRotation` _returnvalue (`KismetMathLibrary.MakeRotator` 0.0)))
      (:`<`
        (`Controller.SetControlRotation` _returnvalue (`KismetMathLibrary.MakeRotator` 0.0 0.0 180.0))))))

(event `InputAction|SwapNextDice`
  (params (Key :type "Key Structure"))
  (bind _availabledices (`self.AvailableDices`))
  (bind _returnvalue (+ (`KismetArrayLibrary.Array_Find` _availabledices (`self.CurrentDice`)) 1))
  ;[1 1 1] Inputs
  (:`Pressed`
    (bind _yes (`self.CanCurrentlySwap`))
    (if _yes
      (`self.SetDice` (`|GetArrayItem` (`self.AvailableDices`) (`KismetMathLibrary.SelectInt` 0 _returnvalue (>= _returnvalue (`KismetArrayLibrary.Array_Length` _availabledices))))))))

(event `InputAction|SwapPrevDice`
  (params (Key :type "Key Structure"))
  (bind _availabledices (`self.AvailableDices`))
  (bind _returnvalue (- (`KismetArrayLibrary.Array_Find` _availabledices (`self.CurrentDice`)) 1))
  ;[1 1 1] Inputs
  (:`Pressed`
    (bind _yes (`self.CanCurrentlySwap`))
    (if _yes
      (`self.SetDice` (`|GetArrayItem` (`self.AvailableDices`) (`KismetMathLibrary.SelectInt` (- (`KismetArrayLibrary.Array_Length` _availabledices) 1) _returnvalue (< _returnvalue 0)))))))

(event `InputAction|UseSkill`
  (params (Key :type "Key Structure"))
  ;[1 1 1] Inputs
  (:`Pressed`
    (`self.UseCurrentSkill`)))

(event `self.OnLanded`
  (params (Hit :type "HitResult Structure (by ref)"))
  ;[1 1 1] BigJump
  (set `self.JumpMaxCount` (`KismetMathLibrary.SelectInt` 2 1 (== (`self.CurrentDice`) 6)))
  (set `CharacterMovementComponent.JumpZVelocity` (`self.OriginalJumpZVelocity`) (`self.CharacterMovement`)))

(fn `CanCurrentlySwap`
  (returns (Yes :type Boolean))
  (return (and (> (`KismetArrayLibrary.Array_Length` (`self.AvailableDices`)) 1) (<= (`self.StealthCurrentTime`) 0.0) (<= (`self.DashCurrentTime`) 0.0))))

(fn `CanDash`
  (returns (NewParam :type Boolean))
  (return (`KismetArrayLibrary.Array_Contains` (`self.AvailableDices`) 10)))

(fn `CanDoubleJump`
  (returns (NewParam :type Boolean))
  (return (`KismetArrayLibrary.Array_Contains` (`self.AvailableDices`) 6)))

(fn `CanPiouPiou`
  (returns (NewParam :type Boolean))
  (return (`KismetArrayLibrary.Array_Contains` (`self.AvailableDices`) 20)))

(fn `CanSlowDown`
  (returns (NewParam :type Boolean))
  (return (`KismetArrayLibrary.Array_Contains` (`self.AvailableDices`) 8)))

(fn `CanStealth`
  (returns (NewParam :type Boolean))
  (return (`KismetArrayLibrary.Array_Contains` (`self.AvailableDices`) 12)))

(fn `DiceNumberToId`
  (params (Number :type Integer))
  (returns (Id :type Integer))
  (return (`.DiceIndex_24_04B80ABF469124BD46DBD1822D084F0A` (break `/Game/Player/DiceParameters` (`BlueprintMapLibrary.Map_Find` (`self.DiceParametersArray`) Number)))))

(fn `EnableDice`
  (params (Number :type Integer) (Enable :type Boolean))
  (bind _capsulecomponent (`self.CapsuleComponent`))
  (bind (_value _returnvalue) (`BlueprintMapLibrary.Map_Find` (`self.DiceParametersArray`) Number))
  (bind (_leftarmpositon _rightarmposition _legpostion _capsulehalfheight _capsuleradius) (break `/Game/Player/DiceParameters` _value))
  (if _returnvalue
    (`self.UnlockSkill` Enable Number)
    (bind _fbdice (`self.GetFlipBookForDice` Number))
    (`SceneComponent.SetVisibility` _fbdice Enable false)
    (if Enable
      (`SceneComponent.K2_SetRelativeLocation` (`self.LeftArm`) _leftarmpositon false false)
      (`SceneComponent.K2_SetRelativeLocation` (`self.RightArm`) _rightarmposition false false)
      (`SceneComponent.K2_SetRelativeLocation` (`self.Sprite`) _legpostion false false)
      (`CapsuleComponent.SetCapsuleRadius` _capsulecomponent _capsuleradius true)
      (`CapsuleComponent.SetCapsuleHalfHeight` _capsulecomponent _capsulehalfheight true))))

(fn `GainDice`
  (params (DiceNumber :type Integer))
  (if (not (`KismetArrayLibrary.Array_Contains` (`self.AvailableDices`) DiceNumber))
    (`/Game/UI/BP_HUD.GainPower` (`self.HUD`) DiceNumber)
    (for (_array_element _array_index) (`self.AvailableDices`)
      (if (> _array_element DiceNumber)
        (`KismetArrayLibrary.Array_Insert` (`self.AvailableDices`) DiceNumber _array_index)
        (return)))
    (`KismetArrayLibrary.Array_Add` (`self.AvailableDices`) DiceNumber)))

(fn `GetFlipBookForDice`
  (params (DiceNumer :type Integer))
  (returns (FBDice :type "PaperFlipbookComponent Object Reference"))
  (return (select `bool` (== DiceNumer 4) :`false` (select `bool` (== DiceNumer 6) :`false` (select `bool` (== DiceNumer 8) :`false` (select `bool` (== DiceNumer 10) :`false` (select `bool` (== DiceNumer 12) :`false` (select `bool` (== DiceNumer 20) :`true` (`self.Dice20`)) :`true` (`self.Dice12`)) :`true` (`self.Dice10`)) :`true` (`self.Dice8`)) :`true` (`self.Dice6`)) :`true` (`self.Dice4`))))

(fn `GetMissingDicesList`
  (returns (MissingDiceIDs :type "Array of Integer"))
  (locals (MissingDices :type "Array of Integer"))
  (bind _keys (`BlueprintMapLibrary.Map_Keys` (`self.DiceParametersArray`)))
  (for _array_element _keys
    (if (== (`KismetArrayLibrary.Array_Find` (`self.AvailableDices`) _array_element) -1)
      (bind (_value _returnvalue) (`BlueprintMapLibrary.Map_Find` (`self.DiceParametersArray`) _array_element))
      (if _returnvalue
        (`KismetArrayLibrary.Array_Add` (`local.MissingDices`) (`.DiceIndex_24_04B80ABF469124BD46DBD1822D084F0A` (break `/Game/Player/DiceParameters` _value))))))
  (return (`local.MissingDices`)))

(fn `IdToDiceNumber`
  (params (ID :type Integer))
  (returns (Number :type Integer))
  (bind _values (`BlueprintMapLibrary.Map_Values` (`self.DiceParametersArray`)))
  (for (_array_element _array_index) _values
    (if (== (`.DiceIndex_24_04B80ABF469124BD46DBD1822D084F0A` (break `/Game/Player/DiceParameters` _array_element)) ID)
      (bind _keys (`BlueprintMapLibrary.Map_Keys` (`self.DiceParametersArray`)))
      (return (`|GetArrayItem` _keys _array_index))))
  (return 0))

(fn `IsDashCoolingDown`
  (returns (NewParam :type Boolean))
  (return (> (`self.CooldownDash`) 0.0)))

(fn `IsProjectileCoolingDown`
  (returns (NewParam :type Boolean))
  (return (> (`self.CooldownProjectile`) 0.0)))

(fn `IsSlowDownCoolingDown`
  (returns (NewParam :type Boolean))
  (return (> (`self.CooldownSlowDown`) 0.0)))

(fn `IsStealthCoolingDown`
  (returns (NewParam :type Boolean))
  (return (> (`self.CooldownStealth`) 0.0)))

(fn `IsStealthy`
  (returns (out :type Boolean))
  (return (> (`self.StealthCurrentTime`) 0.0)))

(fn `Lose Current Dice`
  (locals (DiceNumberToRemove :type Integer))
  (bind _availabledices (`self.AvailableDices`))
  (bind _returnvalue (- (`KismetArrayLibrary.Array_Find` _availabledices (`self.CurrentDice`)) 1))
  ;[1 1 1] Stop powers
  (if (> (`self.DashCurrentTime`) 0.0)
    (set `self.DashCurrentTime` 0.01))
  (if (> (`self.StealthCurrentTime`) 0.0)
    (set `self.StealthCurrentTime` 0.01))
  (bind _asbp_game_instance (cast `/Game/BP_GameInstance` (`GameplayStatics.GetGameInstance`))
    (:`then`
      (`/Game/Runner/BP_RunnerManager.OnInterruptSlowDown` (`/Game/BP_GameInstance.RunnerManager` _asbp_game_instance))
      (`/Game/Daron/BP_Daron.OnInterruptSlowDown` (`/Game/BP_GameInstance.DaronObject` _asbp_game_instance)))
    (:`CastFailed`
      _))
  ;[1 1 1] Check lost
  (if (== (`KismetArrayLibrary.Array_Length` (`self.AvailableDices`)) 1)
    (`self.LoseGame`)
    (else
      (`/Game/UI/BP_HUD.LosePower` (`self.HUD`) (`self.CurrentDice`))
      ;[1 1 1] Remove dice
      (set `local.DiceNumberToRemove` (`self.CurrentDice`))
      (`self.SetDice` (`|GetArrayItem` _availabledices (`KismetMathLibrary.SelectInt` _returnvalue (- (`KismetArrayLibrary.Array_Length` _availabledices) 1) (>= _returnvalue 0))))
      (`KismetArrayLibrary.Array_RemoveItem` (`self.AvailableDices`) (`local.DiceNumberToRemove`)))))

(fn `LoseGame`
  (bind _endscreen (`self.EndScreen`))
  (`GameplayStatics.SetGamePaused` true)
  (`/Game/UI/Bp_EndScreen.OnGameOver` _endscreen)
  (`UserWidget.AddToViewport` _endscreen 0)
  (`/Game/UI/Bp_EndScreen.OnShow` _endscreen))

(fn `OnWin`
  (bind _endscreen (`self.EndScreen`))
  (`GameplayStatics.SetGamePaused` true)
  (`UserWidget.AddToViewport` _endscreen 0)
  (`Widget.SetFocus` _endscreen)
  (`/Game/UI/Bp_EndScreen.OnShow` _endscreen))

(fn `SetDice`
  (params (DiceNumber :type Integer))
  (`self.EnableDice` (`self.CurrentDice`))
  (bind _output_get (set `self.CurrentDice` DiceNumber))
  (`self.EnableDice` _output_get true))

(fn `UnlockSkill`
  (params (Unlock :type Boolean) (DiceNumber :type Integer))
  (if (== DiceNumber 6)
    ;[1 1 1] D6
    (set `self.JumpMaxCount` (`KismetMathLibrary.SelectInt` 2 1 Unlock))))

(fn `UpdateCooldowns`
  (params (Dt :type "Float (double-precision)"))
  (bind _cooldownprojectile (`self.CooldownProjectile`))
  (bind _cooldownstealth (`self.CooldownStealth`))
  (bind _cooldownslowdown (`self.CooldownSlowDown`))
  (bind _cooldowndash (`self.CooldownDash`))
  (if (> _cooldownprojectile 0.0)
    (bind _output_get (set `self.CooldownProjectile` (- _cooldownprojectile Dt)))
    (`/Game/UI/BP_HUD.SetPercentForDiceAbility` (`self.HUD`) (- 1.0 (/ _output_get (`self.CooldownProjectileMax`))) 20))
  (if (> _cooldownslowdown 0.0)
    (bind _output_get_2 (set `self.CooldownSlowDown` (- _cooldownslowdown Dt)))
    (`/Game/UI/BP_HUD.SetPercentForDiceAbility` (`self.HUD`) (- 1.0 (/ _output_get_2 (`self.CooldownSlowDownMax`))) 8))
  (if (> _cooldowndash 0.0)
    (bind _output_get_3 (set `self.CooldownDash` (- _cooldowndash Dt)))
    (`/Game/UI/BP_HUD.SetPercentForDiceAbility` (`self.HUD`) (- 1.0 (/ _output_get_3 (`self.CooldownDashMax`))) 10))
  (if (> _cooldownstealth 0.0)
    (bind _output_get_4 (set `self.CooldownStealth` (- _cooldownstealth Dt)))
    (`/Game/UI/BP_HUD.SetPercentForDiceAbility` (`self.HUD`) (- 1.0 (/ _output_get_4 (`self.CooldownStealthMax`))) 12))
  (`/Game/UI/BP_HUD.SetPercentForDiceAbility` (`self.HUD`) 0.0 4)
  (`/Game/UI/BP_HUD.SetPercentForDiceAbility` (`self.HUD`) (`KismetMathLibrary.SelectFloat` 1.0 0.0 (or (`self.CanJump`) (!= (`self.CurrentDice`) 6))) 6))

(fn `UseCurrentSkill`
  (bind _returnvalue_location (`KismetMathLibrary.BreakTransform` (`self.GetTransform`)))
  (bind (_returnvalue_roll _returnvalue_pitch _returnvalue_yaw) (`KismetMathLibrary.BreakRotator` (`self.GetControlRotation`)))
  (bind _charactermovement (`self.CharacterMovement`))
  (bind _rightarm (`self.RightArm`))
  (bind _sprite (`self.Sprite`))
  (bind _leftarm (`self.LeftArm`))
  (bind _value (`BlueprintMapLibrary.Map_Find` (`self.DiceParametersArray`) 10))
  (bind (_x _y _z) (`KismetMathLibrary.BreakVector3f` (break `/Game/Player/DiceParameters` _value)))
  (bind (_x_2 _y_2 _z_2) (`KismetMathLibrary.BreakVector3f` (`.RightArmPosition_9_4A7DAD8C4587A3831790768D12833F1F` (break `/Game/Player/DiceParameters` _value))))
  (if (== (`self.CurrentDice`) 20)
    ;[1 1 1] D20 - Pioupiou
    (if (<= (`self.CooldownProjectile`) 0.0)
      (bind _returnvalue (`|SpawnActorFromClass` "/Game/Projectile/BP_Projectile.BP_Projectile_C" (`KismetMathLibrary.MakeTransform` (+ _returnvalue_location (-32.0 0.0 24.0)) (struct :`Pitch` 90.0) (2.0 2.0 2.0)) "AlwaysSpawn" "OverrideRootScale" null null))
      (`/Engine/EditorBlueprintResources/StandardMacros.IsValid` _returnvalue
        (:`Is Valid`
          (set `/Game/Projectile/BP_Projectile.Direction` (-200.0 0.0 0.0) _returnvalue)
          (`/Game/Projectile/BP_Projectile.Init` _returnvalue)
          (set `self.CooldownProjectile` (`self.CooldownProjectileMax`))))
      (else
        (`KismetSystemLibrary.PrintString` "PiouPiou is cooling down!")))
    (elif (== (`self.CurrentDice`) 8)
      ;[1 1 1] D8 - SlowDown
      (if (<= (`self.CooldownSlowDown`) 0.0)
        (bind _asbp_game_instance (cast `/Game/BP_GameInstance` (`GameplayStatics.GetGameInstance`)))
        (`/Game/Runner/BP_RunnerManager.OnSlowDown` (`/Game/BP_GameInstance.RunnerManager` _asbp_game_instance) 5.0)
        (`/Game/Daron/BP_Daron.OnSlowDown` (`/Game/BP_GameInstance.DaronObject` _asbp_game_instance) 5.0)
        (set `self.CooldownSlowDown` (`self.CooldownSlowDownMax`))
        (else
          (`KismetSystemLibrary.PrintString` "SlowDown is cooling down!")))
      (elif (== (`self.CurrentDice`) 10)
        ;[1 1 1] D10 - Dash
        (if (<= (`self.CooldownDash`) 0.0)
          (set `self.DashCurrentTime` (`self.DashDuration`))
          (`MovementComponent.StopMovementImmediately` _charactermovement)
          (set `CharacterMovementComponent.GravityScale` 0.001 _charactermovement)
          (`self.LaunchCharacter` (`KismetMathLibrary.MakeVector` (* (`KismetMathLibrary.SelectFloat` -1.0 1.0 (> _returnvalue_yaw 0.0)) (`self.DashSpeed`))))
          (set `self.CooldownDash` (`self.CooldownDashMax`))
          (`PaperFlipbookComponent.SetFlipbook` _sprite "/Game/Dice_sprite/FB_LegsDash.FB_LegsDash")
          (`SceneComponent.K2_SetRelativeLocation` _sprite (`KismetMathLibrary.MakeVector` (+ (.x (`.LegPostion_21_4465FA6C4BA7FE0268173FB8DA4CB8B8` (break `/Game/Player/DiceParameters` _value))) -4.0) (.y (`.LegPostion_21_4465FA6C4BA7FE0268173FB8DA4CB8B8` (break `/Game/Player/DiceParameters` _value))) (.z (`.LegPostion_21_4465FA6C4BA7FE0268173FB8DA4CB8B8` (break `/Game/Player/DiceParameters` _value)))) false false)
          (`PaperFlipbookComponent.SetFlipbook` _leftarm "/Game/Dice_sprite/FB_ArmDash.FB_ArmDash")
          (`SceneComponent.K2_SetRelativeLocation` _leftarm (`KismetMathLibrary.MakeVector` (+ _x 3.0) _y _z) false false)
          (`PaperFlipbookComponent.SetFlipbook` _rightarm "/Game/Dice_sprite/FB_ArmDash.FB_ArmDash")
          (`SceneComponent.K2_SetRelativeLocation` _rightarm (`KismetMathLibrary.MakeVector` (+ _x_2 -18.0) (+ _y_2 -4.0) _z_2) false false)
          (else
            (`KismetSystemLibrary.PrintString` "Dash is cooling down!")))
        (elif (== (`self.CurrentDice`) 12)
          ;[1 1 1] D12 - Stealth
          (if (<= (`self.CooldownStealth`) 0.0)
            (set `self.StealthCurrentTime` (`self.StealthDuration`))
            (`SceneComponent.SetVisibility` (`self.Box`) true true)
            (set `self.CooldownStealth` (`self.CooldownStealthMax`))
            (`PrimitiveComponent.SetCollisionResponseToChannel` (`self.CapsuleComponent`) "ECC_GameTraceChannel2" "ECR_Ignore")
            (else
              (`KismetSystemLibrary.PrintString` "Stealth is cooling down!")))
          (elif (== (`self.CurrentDice`) 6)
            ;[1 1 1] D6 - SuperJump
            (if (`self.CanJump`)
              (set `CharacterMovementComponent.JumpZVelocity` (* (`self.OriginalJumpZVelocity`) 1.5) (`self.CharacterMovement`))
              (`self.Jump`)
              (set `self.JumpMaxCount` 1))))))))

(fn `UserConstructionScript`)