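; BP_Background is a parallax scrolling backdrop for the runner game.
; Each tick it shifts the Sky and Background components along relative X, against the RunnerManager's BlockMoveSpeed read from BP_GameInstance.
; Sky moves at half the rate of Background to suggest depth.
; Both offsets wrap with a 128-unit modulo, so the scroll repeats indefinitely.
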(event `self.ReceiveTick`
  (params (DeltaSeconds :type "Float (single-precision)"))
  (bind _background (`self.Background`))
  (bind _sky (`self.Sky`))
  (bind (_relativelocation_x _relativelocation_y _relativelocation_z) (`KismetMathLibrary.BreakVector` (`SceneComponent.RelativeLocation` _background)))
  (bind (_relativelocation_x_2 _relativelocation_y_2 _relativelocation_z_2) (`KismetMathLibrary.BreakVector` (`SceneComponent.RelativeLocation` _sky)))
  (bind _asbp_game_instance (cast `/Game/BP_GameInstance` (`GameplayStatics.GetGameInstance`)))
  (bind _blockmovespeed (`/Game/Runner/BP_RunnerManager.BlockMoveSpeed` (`/Game/BP_GameInstance.RunnerManager` _asbp_game_instance)))
  (`SceneComponent.K2_SetRelativeLocation` _sky (`KismetMathLibrary.MakeVector` (mod (+ (* _blockmovespeed DeltaSeconds -0.025) _relativelocation_x_2) 128.0) _relativelocation_y_2 _relativelocation_z_2) false false)
  (`SceneComponent.K2_SetRelativeLocation` _background (`KismetMathLibrary.MakeVector` (mod (+ (* _blockmovespeed DeltaSeconds -0.05) _relativelocation_x) 128.0) _relativelocation_y _relativelocation_z) false false))

(fn `UserConstructionScript`)